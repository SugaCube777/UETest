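; BP_Water is a stylized ocean actor with a water surface plane, an underwater plane and a caustics decal.
; Its construction script applies the configurable materials to all three and scales the actor and decal by OceanScale.
; On actor overlap, it writes the water plane's doubled world location to the "Water Height" parameter in MPC_Water.
; An underwater post-process setup exists in the construction script but is disconnected and never runs.
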(event `self.ReceiveActorBeginOverlap`
  (params (OtherActor :type "Actor Object Reference"))
  (`KismetMaterialLibrary.SetVectorParameterValue` "/Game/WaterStylizedNew/Material/MaterialParameter/MPC_Water.MPC_Water" "Water Height" (`KismetMathLibrary.Conv_VectorToLinearColor` (* (`SceneComponent.K2_GetComponentLocation` (`self.WaterPlane`)) 2.0))))

(fn `UserConstructionScript`
  (bind _oceanscale (`self.OceanScale`))
  (`PrimitiveComponent.SetMaterial` (`self.UnderWaterPlane`) 0 (`self.Underwater Material`))
  (`PrimitiveComponent.SetMaterial` (`self.WaterPlane`) 0 (`self.WaterMaterial`))
  (`DecalComponent.SetDecalMaterial` (`self.Decal`) (`self.CausticsDecalMaterial`))
  (`self.SetActorScale3D` _oceanscale)
  (`SceneComponent.SetWorldScale3D` (`self.Decal`) _oceanscale))