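; Configurable waterfall actor combining a static mesh with Foam, Drop and Drop1 effect components.
; The construction script passes Width to all three effects and scales the mesh by Width horizontally and ScaleZ vertically.
; It moves Drop up in proportion to ScaleZ and applies the min/max colors to Foam and Drop, but not Drop1.
; The event graph holds only disabled placeholder events, so the Blueprint adds no runtime logic.
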(fn `UserConstructionScript`
  (bind _foam (`self.Foam`))
  (bind _width (`self.Width`))
  (bind _drop (`self.Drop`))
  (`FXSystemComponent.SetFloatParameter` _foam "Width" _width)
  (`FXSystemComponent.SetFloatParameter` _drop "Width" _width)
  (`FXSystemComponent.SetFloatParameter` (`self.Drop1`) "Width" _width)
  (`SceneComponent.SetRelativeScale3D` (`self.StaticMesh`) (`KismetMathLibrary.MakeVector` _width _width (`self.Scale_z`)))
  (`SceneComponent.K2_SetRelativeLocation` (`self.Drop`) (`KismetMathLibrary.MakeVector` 0.0 0.0 (* 950.0 (`self.Scale_z`))) false false)
  (`FXSystemComponent.SetColorParameter` _foam "Color" (`KismetMathLibrary.Conv_ColorToLinearColor` (`self.Color_Min`)))
  (`FXSystemComponent.SetColorParameter` _foam "Color_Max" (`KismetMathLibrary.Conv_ColorToLinearColor` (`self.Color_Max`)))
  (`FXSystemComponent.SetColorParameter` _drop "Color" (`KismetMathLibrary.Conv_ColorToLinearColor` (`self.Color_Min`)))
  (`FXSystemComponent.SetColorParameter` _drop "Color_Max" (`KismetMathLibrary.Conv_ColorToLinearColor` (`self.Color_Max`))))